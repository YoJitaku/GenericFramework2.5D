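; Base player character Blueprint for a sprite-based character with an orbitable spring-arm camera.
; Helper functions handle camera-relative movement, 45-degree yaw steps turning spring arm and sprite together, and clamped zoom that also remaps camera pitch.
; The Enhanced Input events are empty, and the calls to these helpers and the mapping-context setup are disconnected, so none run here.
; HandleAttack is an empty stub.
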(event Input|EnhancedActionEvents|EnhancedInputActionIA_Move
  (params (ActionValue :type Vector%202D%20Structure) (ElapsedSeconds :type Float%20%28double-precision%29) (TriggeredSeconds :type Float%20%28double-precision%29) (InputAction :type Input%20Action%20Object%20Reference :default "/Game/GenericFramework/EnhancedInputSystem/IA_Character/IA_Move.IA_Move")))

(event Input|EnhancedActionEvents|EnhancedInputActionIA_CameraRotate
  (params (ActionValue :type Float%20%28double-precision%29) (ElapsedSeconds :type Float%20%28double-precision%29) (TriggeredSeconds :type Float%20%28double-precision%29) (InputAction :type Input%20Action%20Object%20Reference :default "/Game/GenericFramework/EnhancedInputSystem/IA_Character/IA_CameraRotate.IA_CameraRotate")))

(event Input|EnhancedActionEvents|EnhancedInputActionIA_SpringArmLength
  (params (ActionValue :type Float%20%28double-precision%29) (ElapsedSeconds :type Float%20%28double-precision%29) (TriggeredSeconds :type Float%20%28double-precision%29) (InputAction :type Input%20Action%20Object%20Reference :default "/Game/GenericFramework/EnhancedInputSystem/IA_Character/IA_SpringArmLength.IA_SpringArmLength")))

(event EventBeginPlay
  (|CallParentFunction))

(fn ConstructionScript
  (|CallParentFunction))

(fn HandleMove
  (params (Axis2D :type Vector%202D%20Structure))
  (bind (_x _y) (Math|Vector2D|BreakVector2D Axis2D))
  (bind _camera (Variables|Default|GetCamera))
  (Pawn|Input|AddMovementInput (+ (* (Math|Vector|GetRightVector _camera) _x) (* _y (Math|Vector|GetForwardVector _camera))) 1.0 false))

(fn HandleAttack)

(fn HandleCameraRotate
  (params (Q&E :type Float%20%28double-precision%29))
  (bind _springarm (Variables|Default|GetSpringArm))
  (bind _sprite (Variables|Default|GetSprite))
  (bind _returnvalue (Transformation|GetWorldRotation _sprite))
  (bind _relativerotation (Variables|/Script/Engine.SceneComponent|GetRelativeRotation _springarm))
  (if (Variables|Default|GetbCanCameraRotate)
    (if (< Q&E 0.0)
      (Variables|Default|SetbCanCameraRotate false)
      (Transformation|SetRelativeRotation _springarm (Math|Rotator|MakeRotator (.roll _relativerotation) (.pitch _relativerotation) (- (.yaw _relativerotation) 45.0)) false false)
      (Transformation|SetWorldRotation _sprite (Math|Rotator|MakeRotator (.roll _returnvalue) (.pitch _returnvalue) (- (.yaw _returnvalue) 45.0)) false false)
      (else
        (Variables|Default|SetbCanCameraRotate false)
        (Transformation|SetRelativeRotation _springarm (Math|Rotator|MakeRotator (.roll _relativerotation) (.pitch _relativerotation) (+ (.yaw _relativerotation) 45.0)) false false)
        (Transformation|SetWorldRotation _sprite (Math|Rotator|MakeRotator (.roll _returnvalue) (.pitch _returnvalue) (+ (.yaw _returnvalue) 45.0)) false false)))
    (Variables|Default|SetbCanCameraRotate true)
    (Variables|Default|SetvSpringArmYawOffset (+ (.yaw (Transformation|GetWorldRotation _springarm)) 9e+01))))

(fn HandleSpringArmLength
  (params (MouseWheelValue :type Float%20%28double-precision%29))
  (bind _springarm (Variables|Default|GetSpringArm))
  (bind _returnvalue (Transformation|GetWorldRotation _springarm))
  (Variables|/Script/Engine.SpringArmComponent|SetTargetArmLength _springarm (Math|Float|Clamp(Float) (+ (* MouseWheelValue 1e+02) (Variables|/Script/Engine.SpringArmComponent|GetTargetArmLength (Variables|Default|GetSpringArm))) 2e+02 1e+03))
  (Development|PrintString (Utilities|String|ToString(Float) (Math|Float|MapRangeClamped (Math|Float|Clamp(Float) (+ (* MouseWheelValue 1e+02) (Variables|/Script/Engine.SpringArmComponent|GetTargetArmLength (Variables|Default|GetSpringArm))) 2e+02 1e+03) 2e+02 1e+03 -5.0 -25.0)))
  (Transformation|SetWorldRotation _springarm (Math|Rotator|MakeRotator (.roll _returnvalue) (Math|Float|MapRangeClamped (Math|Float|Clamp(Float) (+ (* MouseWheelValue 1e+02) (Variables|/Script/Engine.SpringArmComponent|GetTargetArmLength (Variables|Default|GetSpringArm))) 2e+02 1e+03) 2e+02 1e+03 -5.0 -25.0) (.yaw _returnvalue)) false false))