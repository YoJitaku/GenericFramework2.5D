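; BP_IACT_Door is an interactable door actor that toggles between open and closed when Interact fires.
; Interact prints a debug string, then calls OpenDoor or CloseDoor based on the IsOpen flag.
; Each sets the flag, plays a sound at the actor location, and plays or reverses one shared timeline that drives the Door component's relative yaw.
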(event Custom|CloseDoor
  (Variables|Default|SetbIsOpen false)
  (Audio|PlaySoundatLocation "/Engine/VREditor/Sounds/UI/Leave_Simulate.Leave_Simulate" (Transformation|GetActorLocation) "0, 0, 0" 1.0 1.0 0.0 0 0 0 0)
  (bind _zrotation (Timeline|OpenDoorTimeLine Reverse)
    (:Update
      (Transformation|SetRelativeRotation (Variables|Default|GetDoor) (Math|Rotator|MakeRotator 0.0 0.0 _zrotation) false false))))

(event Custom|OpenDoor
  (Variables|Default|SetbIsOpen true)
  (Audio|PlaySoundatLocation "/Engine/VREditor/Sounds/UI/Enter_Simulate.Enter_Simulate" (Transformation|GetActorLocation) "0, 0, 0" 1.0 1.0 0.0 0 0 0 0)
  (bind _zrotation (Timeline|OpenDoorTimeLine Play)
    (:Update
      (Transformation|SetRelativeRotation (Variables|Default|GetDoor) (Math|Rotator|MakeRotator 0.0 0.0 _zrotation) false false))))

(event EventBeginPlay)

(event Collision|EventActorBeginOverlap
  (params (OtherActor :type Actor%20Object%20Reference)))

(event EventTick
  (params (DeltaSeconds :type Float%20%28single-precision%29)))

(event EventInteract
  (params (Interactor :type Actor%20Object%20Reference))
  (Development|PrintString "123123")
  (if (Variables|Default|GetbIsOpen)
    (CallFunction|CloseDoor)
    (else
      (CallFunction|OpenDoor))))

(fn ConstructionScript
  (|CallParentFunction))